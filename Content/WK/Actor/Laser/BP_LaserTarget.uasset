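; BP_LaserTarget is a laser puzzle target that shows whether it is active by changing its color.
; LaserBounce stores the incoming hit response as Active, then passes the laser's color to PuzzleSolved.
; PuzzleSolved creates a new M_FlatCol dynamic material on SMParent at each call, tinted to the laser color when active or grey otherwise.
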(fn ConstructionScript
  (|CallParentFunction))

(fn PuzzleSolved
  (params (Color%20laser :type Linear%20Color%20Structure))
  (bind _returnvalue (Rendering|Material|CreateDynamicMaterialInstance (Variables|Default|GetSM_Parent) 0 "/Game/LevelPrototyping/Materials/M_FlatCol.M_FlatCol" "None" :!class /Script/Engine.PrimitiveComponent))
  (Rendering|Material|SetVectorParameterValue _returnvalue "Base color" (Math|Color|SelectColor Color%20laser "(R=0.365625,G=0.365625,B=0.365625,A=1.000000)" (Variables|Default|GetActive)) :!class /Script/Engine.MaterialInstanceDynamic))

(fn LaserBounce
  (params (P-LaserHits :type BP%20Laser%20Object%20Reference) (P-HitResponses :type Boolean) (P-HitInformation :type Hit%20Result%20Structure))
  (Variables|Default|SetActive P-HitResponses)
  (CallFunction|PuzzleSolved (Variables|/Game/WK/Actor/Laser/BP_LasersParent.BP_LasersParent_C|GetLaser%20colour P-LaserHits))
  (return 0))