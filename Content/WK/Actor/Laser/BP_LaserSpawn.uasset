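; BP_LaserSpawn is an emitter actor that creates a BP_Laser when play begins.
; On BeginPlay it stores a self-reference and its display name as an ID, then spawns the laser at its Arrow component's location using the actor's rotation.
; It passes its laser colour and self-reference to the new laser and records that laser in its ChildLaser collection.
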(event EventBeginPlay
  (Variables|Default|SetSpawn%20referrence self)
  (Variables|Default|SetID (Utilities|GetDisplayName self))
  (bind _returnvalue (Game|SpawnActorfromClass "/Game/WK/Actor/Laser/BP_Laser.BP_Laser_C" (Math|Transform|MakeTransform (Transformation|GetWorldLocation (Variables|Default|GetArrow)) (Transformation|GetActorRotation) "1.000000,1.000000,1.000000") "Undefined" "MultiplyWithRoot" 0 (Variables|Default|GetLaser%20colour) (Variables|Default|GetSpawn%20referrence) 0))
  (Utilities|Array|Add (Variables|Default|GetChild%20laser) _returnvalue))

(fn ConstructionScript
  (|CallParentFunction))