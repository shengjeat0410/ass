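; Laser beam actor that tints its mesh with a configurable colour and reports hits to objects that respond to lasers.
; Each tick a thin box trace runs along the actor's up vector, and the mesh stretches to the hit distance or maximum range.
; Through the BPILasers interface, LaserBounceMessage sends true to a continuously hit actor and false to the previous one when the target changes.
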(event EventBeginPlay
  (CallFunction|ChangeColor))

(event EventTick
  (params (DeltaSeconds :type Float%20%28single-precision%29))
  (CallFunction|SetEndPoint))

(fn ConstructionScript
  (|CallParentFunction))

(fn ChangeColor
  (bind _returnvalue (Rendering|Material|CreateDynamicMaterialInstance (Variables|Default|GetSM_Parent) 0 "/Game/LevelPrototyping/Materials/M_Laser.M_Laser" "None" :!class /Script/Engine.PrimitiveComponent))
  (Rendering|Material|SetVectorParameterValue _returnvalue "Color" (Variables|Default|GetLaser%20colour) :!class /Script/Engine.MaterialInstanceDynamic))

(fn SetEndPoint
  (bind _returnvalue (Transformation|GetActorLocation))
  (bind _returnvalue_2 (Transformation|GetActorUpVector))
  (bind _returnvalue_3 (* _returnvalue_2 2.0))
  (bind _returnvalue_4 (+ _returnvalue _returnvalue_3))
  (bind _outhit (Collision|BoxTraceByChannel _returnvalue_4 (+ _returnvalue_4 (* _returnvalue_2 (Variables|Default|GetL%20range))) "0.500000,0.500000,0.500000" "0, 0, 0" "TraceTypeQuery1" false 0 "None"))
  (bind _output_get (LocalVariables|SetL%20Hit%20Info _outhit))
  (LocalVariables|SetL%20Hit%20Actor (.HitActor (Collision|BreakHitResult _output_get)))
  (Transformation|SetWorldScale3D (Variables|Default|GetSM_Parent) (Math|Vector|MakeVector 0.05 0.05 (Math|Float|SelectFloat (/ (+ (.Distance (Collision|BreakHitResult _output_get)) 1.0) 1e+02) (/ (Variables|Default|GetL%20range) 1e+02) (.bBlockingHit (Collision|BreakHitResult _output_get)))))
  (Utilities|FlowControl|Sequence
    (:then_0
      (if (!= (Variables|Default|Getlast%20hit%20actor) (LocalVariables|GetL%20Hit%20Actor))
        (if (Utilities|DoesObjectImplementInterface (Variables|Default|Getlast%20hit%20actor) "/Game/WK/Actor/Laser/BPI-Lasers.BPI-Lasers_C")
          (Class|BPI-Lasers|LaserBounce(Message) (Variables|Default|Getlast%20hit%20actor) self false (LocalVariables|GetL%20Hit%20Info))
          (Development|PrintString "Hello"))
        (elif (Utilities|DoesObjectImplementInterface (LocalVariables|GetL%20Hit%20Actor) "/Game/WK/Actor/Laser/BPI-Lasers.BPI-Lasers_C")
          (Class|BPI-Lasers|LaserBounce(Message) (LocalVariables|GetL%20Hit%20Actor) self true (LocalVariables|GetL%20Hit%20Info)))))
    (:then_1
      (bind _l_hit_actor (LocalVariables|GetL%20Hit%20Actor)
        (:then
          (Variables|Default|Setlast%20hit%20actor _l_hit_actor))
        (:else)))))