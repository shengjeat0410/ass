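; BP_Conveyor is a conveyor belt actor that carries whatever actors sit on it.
; Each tick it moves every actor overlapping its Box along the Belt's forward vector at Speed, scaled by delta time, using unswept world offsets rather than physics.
; The construction script creates a dynamic material instance on the Belt; a follow-up SetMaterial node is left unconnected.
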(event EventTick
  (params (DeltaSeconds :type Float%20%28single-precision%29))
  (for _array_element (Collision|GetOverlappingActors (Variables|Default|GetBox) 0 :!class /Script/Engine.PrimitiveComponent)
    (Transformation|AddActorWorldOffset _array_element (* (* DeltaSeconds (Variables|Default|GetSpeed)) (Math|Vector|GetForwardVector (Transformation|GetWorldRotation (Variables|Default|GetBelt)))))))

(fn ConstructionScript
  (bind _returnvalue (Rendering|Material|CreateDynamicMaterialInstance (Variables|Default|GetBelt) 0 0 "None" :!class /Script/Engine.PrimitiveComponent)))