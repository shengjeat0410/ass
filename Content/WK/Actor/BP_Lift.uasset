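; BP_Lift is a lift actor whose platform moves vertically in response to switches.
; Switch activated and deactivated events adjust an active-switch count and compare it against the required number.
; Meeting the threshold plays the LiftUpndown timeline, and falling below it reverses the movement.
; The timeline's UpNDown track drives the platform's relative Z location.
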(event Custom|Switch%20deactivated
  (Math|Integer|DecrementInt (Variables|Default|GetSwitch%20active)
    (:%20%20
      (if (>= (Variables|Default|GetSwitch%20active) (Variables|Default|GetSwitch%20needed))
        (bind _upndown (Timeline|Lift%20upndown Play)
          (:Update
            (Transformation|SetRelativeLocation (Variables|Default|GetPlatform) (Math|Vector|MakeVector 0.0 0.0 _upndown) false false)))
        (else
          (Timeline|Lift%20upndown Reverse))))))

(event Custom|Switch%20activated
  (Math|Integer|IncrementInt (Variables|Default|GetSwitch%20active)
    (:%20%20
      (if (>= (Variables|Default|GetSwitch%20active) (Variables|Default|GetSwitch%20needed))
        (bind _upndown (Timeline|Lift%20upndown Play)
          (:Update
            (Transformation|SetRelativeLocation (Variables|Default|GetPlatform) (Math|Vector|MakeVector 0.0 0.0 _upndown) false false)))
        (else
          (Timeline|Lift%20upndown Reverse))))))

(fn ConstructionScript)