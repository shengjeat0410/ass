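; Grapple hook projectile that lets the third-person character swing from surfaces or pull objects tagged Movable.
; A cable links hook to player, with timer-driven visual update and retraction for misses.
; On other hits, Tick applies pendulum and spring forces through CharacterMovement, shortening rope length as the player nears the anchor while grounded or above it.
; Movable hits impulse hook and object toward the player; an impulse-based swing variant is unwired.
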(event OnComponentHit(Sphere)
  (params (HitComponent :type Primitive%20Component%20Object%20Reference) (OtherActor :type Actor%20Object%20Reference) (OtherComp :type Primitive%20Component%20Object%20Reference) (NormalImpulse :type Vector :default "0, 0, 0") (Hit :type Hit%20Result%20Structure%20%28by%20ref%29))
  ;[0.15 0.15 0.15 0.5] 2) Store hit locations, switch cable, change gravity
  ;;[0.15 0.15 0.15 0.5] Pull mechanic with tag: Movable
  (if (not (Actor|ActorHasTag OtherActor "Movable"))
    (bind _output_get (Variables|GrappleComponents|SetGrapple%20hit%20location (.location Hit)))
    (Variables|Default|SetDistance%20of%20rope (Math|Vector|Distance(Vector) (Transformation|GetActorLocation (Variables|ThirdPersomnCharacter|GetBP%20Third%20Person%20Character)) _output_get))
    (Variables|GrappleAddForce|SetApply%20force true) ; Only if using add force
    ;;[0.15 0.15 0.15 0.5] Change cable and stop visual timer
    (Utilities|Time|ClearandInvalidateTimerbyHandle (Variables|GrappleTimers|GetTimer%20grapple%20visual))
    (bind _cable (Variables|GrappleComponents|GetCable)
      (:then
        (Components|DestroyComponent _cable)
        (Rendering|SetVisibility (Variables|GrappleComponents|GetCable1segment) true false))
      (:else))
    (else
      (|Pullobject_2 OtherComp))))

(event Custom|Update%20cable%20visual
  ;[0.15 0.15 0.15 0.5] Update rope length, for realistic visual
  (CallFunction|CableLength)
  ;[0.15 0.15 0.15 0.5] Retract and destroy hook when it hit nothing
  (if true
    (Utilities|FlowControl|DoOnce false
      (:Completed
        (Variables|/Script/Engine.MovementComponent|SetVelocity (Variables|GrappleComponents|GetProjectileMovement) (Utilities|CalculateVelocityChange))
        (Collision|SetCollisionEnabled (Variables|GrappleComponents|GetSphere) "NoCollision")
        (Utilities|FlowControl|Delay 1.0)
        (Utilities|Time|ClearandInvalidateTimerbyHandle (Variables|GrappleTimers|GetTimer%20grapple%20visual))
        (Actor|DestroyActor)
        (Variables|/Game/ThirdPerson/Blueprints/BP_ThirdPersonCharacter.BP_ThirdPersonCharacter_C|SetGrapple%20Active? (Variables|ThirdPersomnCharacter|GetBP%20Third%20Person%20Character) false)))))

(event Custom|Add%20force%20to%20player
  ;[0.15 0.15 0.15 0.5] Add impulse
)

(event EventBeginPlay
  ;[0.15 0.15 0.15 0.5] 1) Cast to player blueprint and attach rope to player
  (bind _asbp_third_person_character (Utilities|Casting|CastToBP_ThirdPersonCharacter (Game|Player|GetPlayerPawn 0)))
  (Variables|ThirdPersomnCharacter|SetBP%20Third%20Person%20Character _asbp_third_person_character)
  (Class|CableComponent|SetAttachEndto (Variables|GrappleComponents|GetCable1segment) (Variables|ThirdPersomnCharacter|GetBP%20Third%20Person%20Character) "Direction of Throw" "None")
  ;[0.15 0.15 0.15 0.5] Update rope length, for realistic visual
  (bind _returnvalue (Utilities|Time|SetTimerbyEvent (delegate Custom|Update%20cable%20visual) 0.001))
  (Variables|GrappleTimers|SetTimer%20grapple%20visual _returnvalue))

(event EventTick
  (params (DeltaSeconds :type Float%20%28single-precision%29))
  ;[0.15 0.15 0.15 0.5] Add force
  (if (Variables|GrappleAddForce|GetApply%20force)
    (CallFunction|SwingForceAddForce)))

(fn ConstructionScript)

(fn CableLength
  (Variables|/Script/CableComponent.CableComponent|SetCableLength (Variables|GrappleComponents|GetCable) (Math|Vector|Distance(Vector) (Transformation|GetActorLocation (Variables|ThirdPersomnCharacter|GetBP%20Third%20Person%20Character)) (Transformation|GetWorldLocation (Variables|GrappleComponents|GetGrapple_mesh)))))

(fn Cable1SegmentLength
  (Variables|/Script/CableComponent.CableComponent|SetCableLength (Variables|GrappleComponents|GetCable1segment) (Math|Vector|Distance(Vector) (Transformation|GetActorLocation (Variables|ThirdPersomnCharacter|GetBP%20Third%20Person%20Character)) (Variables|GrappleComponents|GetGrapple%20hit%20location))))

(fn CancelGrapple
  ;[0.15 0.15 0.15 0.5] Stop timer and reset variables
  (Utilities|Time|ClearandInvalidateTimerbyHandle (Variables|GrappleTimers|GetGrapple%20hooked%20timer))
  (Variables|/Script/Engine.CharacterMovementComponent|SetGravityScale (Variables|/Script/Engine.Character|GetCharacterMovement (Variables|ThirdPersomnCharacter|GetBP%20Third%20Person%20Character)) 2.0)
  (Actor|DestroyActor)
  (Variables|/Game/ThirdPerson/Blueprints/BP_ThirdPersonCharacter.BP_ThirdPersonCharacter_C|SetGrapple%20Active? (Variables|ThirdPersomnCharacter|GetBP%20Third%20Person%20Character) false)
  (Variables|GrappleAddForce|SetApply%20force false))

(fn SwingForceAddForce
  (bind _grapple_hit_location (Variables|GrappleComponents|GetGrapple%20hit%20location))
  (bind _bp_third_person_character (Variables|ThirdPersomnCharacter|GetBP%20Third%20Person%20Character))
  (bind _grapple_hit_location_2 (Variables|GrappleComponents|GetGrapple%20hit%20location))
  (bind _bp_third_person_character_2 (Variables|ThirdPersomnCharacter|GetBP%20Third%20Person%20Character))
  (bind _grapple_hit_location_3 (Variables|GrappleComponents|GetGrapple%20hit%20location))
  (bind _bp_third_person_character_3 (Variables|ThirdPersomnCharacter|GetBP%20Third%20Person%20Character))
  (bind _returnvalue (Transformation|GetActorLocation _bp_third_person_character_2))
  (bind _returnvalue_2 (Transformation|GetActorLocation _bp_third_person_character_3))
  (bind _returnvalue_3 (Transformation|GetActorLocation _bp_third_person_character))
  (bind _returnvalue_4 (Math|Vector|Distance(Vector) _returnvalue _grapple_hit_location_3))
  (bind _returnvalue_5 (Math|Vector|Distance(Vector) _returnvalue_3 _grapple_hit_location_2))
  (bind _returnvalue_6 (- _returnvalue_2 _grapple_hit_location))
  (if (Utilities|CanSwing)
    _
    (else
      ;[0.15 0.15 0.15 0.5] Force applied only if below hook point
      (Physics|AddForce (Variables|/Script/Engine.Character|GetCharacterMovement (Variables|ThirdPersomnCharacter|GetBP%20Third%20Person%20Character)) (* (* (Math|Vector|DotProduct (Variables|/Script/Engine.MovementComponent|GetVelocity (Variables|/Script/Engine.Character|GetCharacterMovement _bp_third_person_character_3)) _returnvalue_6) (Math|Vector|Normalize _returnvalue_6)) -1.0))))
  ;[0.15 0.15 0.15 0.5] Spring force always active
  (Physics|AddForce (Variables|/Script/Engine.Character|GetCharacterMovement (Variables|ThirdPersomnCharacter|GetBP%20Third%20Person%20Character)) (* (* (Math|Float|SelectFloat 0.0 (Variables|Default|GetSpring%20force%20add%20force) (and (Utilities|CanSwing) (<= _returnvalue_5 (Variables|Default|GetDistance%20of%20rope)))) (- (Variables|Default|GetDistance%20of%20rope) _returnvalue_5)) (Math|Vector|Normalize (- (Transformation|GetActorLocation (Variables|ThirdPersomnCharacter|GetBP%20Third%20Person%20Character)) (Variables|GrappleComponents|GetGrapple%20hit%20location)))))
  ;[0.15 0.15 0.15 0.5] Only update distance to make rope shorter
  (if (and (<= _returnvalue_4 (Variables|Default|GetDistance%20of%20rope)) (Utilities|CanSwing))
    (Variables|Default|SetDistance%20of%20rope _returnvalue_4)))

(fn SwingForceAddImpulse
  (bind _grapple_hit_location (Variables|GrappleComponents|GetGrapple%20hit%20location))
  (bind _bp_third_person_character (Variables|ThirdPersomnCharacter|GetBP%20Third%20Person%20Character))
  (bind _grapple_hit_location_2 (Variables|GrappleComponents|GetGrapple%20hit%20location))
  (bind _bp_third_person_character_2 (Variables|ThirdPersomnCharacter|GetBP%20Third%20Person%20Character))
  (bind _grapple_hit_location_3 (Variables|GrappleComponents|GetGrapple%20hit%20location))
  (bind _bp_third_person_character_3 (Variables|ThirdPersomnCharacter|GetBP%20Third%20Person%20Character))
  (bind _returnvalue (Transformation|GetActorLocation _bp_third_person_character_2))
  (bind _returnvalue_2 (Transformation|GetActorLocation _bp_third_person_character_3))
  (bind _returnvalue_3 (Transformation|GetActorLocation _bp_third_person_character))
  (bind _returnvalue_4 (Math|Vector|Distance(Vector) _returnvalue _grapple_hit_location_3))
  (bind _returnvalue_5 (Math|Vector|Distance(Vector) _returnvalue_3 _grapple_hit_location_2))
  (bind _returnvalue_6 (- _returnvalue_2 _grapple_hit_location))
  (if (Utilities|CanSwing)
    _
    (else
      ;[0.15 0.15 0.15 0.5] Force applied only if below hook point
      (Physics|AddImpulse (Variables|/Script/Engine.Character|GetCharacterMovement (Variables|ThirdPersomnCharacter|GetBP%20Third%20Person%20Character)) (* (* (Math|Vector|DotProduct (Variables|/Script/Engine.MovementComponent|GetVelocity (Variables|/Script/Engine.Character|GetCharacterMovement _bp_third_person_character_3)) _returnvalue_6) (Math|Vector|Normalize _returnvalue_6)) -0.004) false)))
  ;[0.15 0.15 0.15 0.5] Spring force always active
  (Physics|AddImpulse (Variables|/Script/Engine.Character|GetCharacterMovement (Variables|ThirdPersomnCharacter|GetBP%20Third%20Person%20Character)) (* (* (Math|Float|SelectFloat 0.0 (Variables|Default|GetSpring%20force%20add%20impulse) (and (Utilities|CanSwing) (<= _returnvalue_5 (Variables|Default|GetDistance%20of%20rope)))) (- (Variables|Default|GetDistance%20of%20rope) _returnvalue_5)) (Math|Vector|Normalize (- (Transformation|GetActorLocation (Variables|ThirdPersomnCharacter|GetBP%20Third%20Person%20Character)) (Variables|GrappleComponents|GetGrapple%20hit%20location)))) false)
  ;[0.15 0.15 0.15 0.5] Only update distance to make rope shorter
  (if (and (<= _returnvalue_4 (Variables|Default|GetDistance%20of%20rope)) (Utilities|CanSwing))
    (Variables|Default|SetDistance%20of%20rope _returnvalue_4)))