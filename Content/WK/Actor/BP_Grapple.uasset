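; Grappling hook projectile that pulls the player toward "Anchor" actors or yanks "Movable" objects toward the player.
; Timers resize the attached cables and, on anchor hits, apply impulses blending camera and hook directions under altered gravity until a timed cancel.
; Movable hits receive a delayed impulse toward the player.
; A distance check gates retracting and destroying a missed hook, and every exit clears the character's GrappleActive flag.
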(event OnComponentHit(Sphere)
  (params (HitComponent :type Primitive%20Component%20Object%20Reference) (OtherActor :type Actor%20Object%20Reference) (OtherComp :type Primitive%20Component%20Object%20Reference) (NormalImpulse :type Vector :default "0, 0, 0") (Hit :type Hit%20Result%20Structure%20%28by%20ref%29))
  ;[0.15 0.15 0.15 0.5] 2) Store hit locations, switch cable, change gravity
  ;;[0.15 0.15 0.15 0.5] Pull player to Anchor using tag
  (if (Actor|ActorHasTag OtherActor "Anchor")
    (Development|PrintString "Anchor")
    (Variables|GrappleVariables|SetGrapple%20hit%20location (.location Hit))
    ;;[0.15 0.15 0.15 0.5] Change cable and stop visual timer
    (Utilities|Time|ClearandInvalidateTimerbyHandle (Variables|GrappleTimers|GetTimer%20grapple%20visual))
    (bind _cable (Variables|Grapplecomponents|GetCable)
      (:then
        (Components|DestroyComponent _cable)
        (Rendering|SetVisibility (Variables|Grapplecomponents|GetCable1segment) true false)
        ;;[0.15 0.15 0.15 0.5] Gravity
        (Variables|/Script/Engine.CharacterMovementComponent|SetGravityScale (Variables|/Script/Engine.Character|GetCharacterMovement (Variables|ThirdPersomnCharacter|GetBP%20Third%20Person%20Character)) (Variables|GrappleVariables|GetGrapple%20gravity))
        ;[0.15 0.15 0.15 0.5] Timer that drives length of rope and force (if add impulse)
        (bind _returnvalue (Utilities|Time|SetTimerbyEvent (delegate Custom|Add%20force%20to%20player) 0.001 true))
        (Variables|GrappleTimers|SetGrapple%20hooked%20timer _returnvalue)
        ;[0.15 0.15 0.15 0.5] Limit grapple by duration
        (Utilities|FlowControl|Delay 3.0)
        (CallFunction|CancelGrapple))
      (:else))
    (else
      ;;[0.15 0.15 0.15 0.5] Pull object with tag: Movable towards player
      (if (Actor|ActorHasTag OtherActor "Movable")
        (Development|PrintString "Movable")
        (|Pullobject_2 OtherComp)
        (else
          ;[0.15 0.15 0.15 0.5] Retract and destroy hook when it no tag (break this if u want the player use grapple to cheat)
          (if (Utilities|CheckDistancetoPlayer)
            (Utilities|FlowControl|DoOnce false
              (:Completed
                (Variables|/Script/Engine.MovementComponent|SetVelocity (Variables|Grapplecomponents|GetProjectileMovement) (Utilities|CalculateVelocityChange))
                (Collision|SetCollisionEnabled (Variables|Grapplecomponents|GetSphere) "PhysicsOnly")
                (Utilities|FlowControl|Delay 0.1)
                (Utilities|Time|ClearandInvalidateTimerbyHandle (Variables|GrappleTimers|GetTimer%20grapple%20visual))
                (Actor|DestroyActor)
                (Variables|/Game/ThirdPerson/Blueprints/BP_ThirdPersonCharacter.BP_ThirdPersonCharacter_C|SetGrapple%20Active? (Variables|ThirdPersomnCharacter|GetBP%20Third%20Person%20Character) false)))))))))

(event Custom|Update%20cable%20visual
  ;[0.15 0.15 0.15 0.5] Update rope length, for realistic visual
  (CallFunction|CableLength)
  ;[0.15 0.15 0.15 0.5] Retract and destroy hook when it hit nothing
  (if (Utilities|CheckDistancetoPlayer)
    (Utilities|FlowControl|DoOnce false
      (:Completed
        (Variables|/Script/Engine.MovementComponent|SetVelocity (Variables|Grapplecomponents|GetProjectileMovement) (Utilities|CalculateVelocityChange))
        (Collision|SetCollisionEnabled (Variables|Grapplecomponents|GetSphere) "NoCollision")
        (Utilities|FlowControl|Delay 1.0)
        (Utilities|Time|ClearandInvalidateTimerbyHandle (Variables|GrappleTimers|GetTimer%20grapple%20visual))
        (Actor|DestroyActor)
        (Variables|/Game/ThirdPerson/Blueprints/BP_ThirdPersonCharacter.BP_ThirdPersonCharacter_C|SetGrapple%20Active? (Variables|ThirdPersomnCharacter|GetBP%20Third%20Person%20Character) false)))))

(event Custom|Add%20force%20to%20player
  ;[0.15 0.15 0.15 0.5] Add impulse
  (CallFunction|Cable1SegmentLength)
  (CallFunction|ForceDirectionwithAddImpulse))

(event EventBeginPlay
  ;[0.15 0.15 0.15 0.5] 1) Cast to player blueprint and attach rope to player
  (bind _asbp_third_person_character (Utilities|Casting|CastToBP_ThirdPersonCharacter (Game|Player|GetPlayerPawn 0)))
  (Variables|ThirdPersomnCharacter|SetBP%20Third%20Person%20Character _asbp_third_person_character)
  (Class|CableComponent|SetAttachEndto (Variables|Grapplecomponents|GetCable1segment) (Variables|ThirdPersomnCharacter|GetBP%20Third%20Person%20Character) "Direction of Throw" "None")
  ;[0.15 0.15 0.15 0.5] Update rope length, for realistic visual
  (bind _returnvalue (Utilities|Time|SetTimerbyEvent (delegate Custom|Update%20cable%20visual) 0.001))
  (Variables|GrappleTimers|SetTimer%20grapple%20visual _returnvalue))

(event EventTick
  (params (DeltaSeconds :type Float%20%28single-precision%29))
  ;[0.15 0.15 0.15 0.5] Add force
)

(fn ConstructionScript)

(fn CableLength
  (Variables|/Script/CableComponent.CableComponent|SetCableLength (Variables|Grapplecomponents|GetCable) (Math|Vector|Distance(Vector) (Transformation|GetActorLocation (Variables|ThirdPersomnCharacter|GetBP%20Third%20Person%20Character)) (Transformation|GetWorldLocation (Variables|Grapplecomponents|GetGrapple_mesh)))))

(fn Cable1SegmentLength
  (Variables|/Script/CableComponent.CableComponent|SetCableLength (Variables|Grapplecomponents|GetCable1segment) (Math|Vector|Distance(Vector) (Transformation|GetActorLocation (Variables|ThirdPersomnCharacter|GetBP%20Third%20Person%20Character)) (Variables|GrappleVariables|GetGrapple%20hit%20location))))

(fn CancelGrapple
  ;[0.15 0.15 0.15 0.5] Stop timer and reset variables
  (Utilities|Time|ClearandInvalidateTimerbyHandle (Variables|GrappleTimers|GetGrapple%20hooked%20timer))
  (Variables|/Script/Engine.CharacterMovementComponent|SetGravityScale (Variables|/Script/Engine.Character|GetCharacterMovement (Variables|ThirdPersomnCharacter|GetBP%20Third%20Person%20Character)) 2.0)
  (Actor|DestroyActor)
  (Variables|/Game/ThirdPerson/Blueprints/BP_ThirdPersonCharacter.BP_ThirdPersonCharacter_C|SetGrapple%20Active? (Variables|ThirdPersomnCharacter|GetBP%20Third%20Person%20Character) false)
  (Variables|GrappleAddForce|SetApply%20force false))

(fn ForceDirectionwithAddForce
  (Physics|AddForce (Variables|/Script/Engine.Character|GetCharacterMovement (Variables|ThirdPersomnCharacter|GetBP%20Third%20Person%20Character)) (+ (* (Math|Vector|Normalize (Math|Vector|GetForwardVector (Variables|/Game/ThirdPerson/Blueprints/BP_ThirdPersonCharacter.BP_ThirdPersonCharacter_C|GetFollowCamera (Variables|ThirdPersomnCharacter|GetBP%20Third%20Person%20Character)))) (Variables|GrappleAddForce|GetCamera%20force%20add%20force)) (* (Math|Vector|Normalize (- (Variables|GrappleVariables|GetGrapple%20hit%20location) (Transformation|GetActorLocation (Variables|ThirdPersomnCharacter|GetBP%20Third%20Person%20Character)))) (Variables|GrappleAddForce|GetHook%20force%20add%20force)))))

(fn ForceDirectionwithAddImpulse
  (Physics|AddImpulse (Variables|/Script/Engine.Character|GetCharacterMovement (Variables|ThirdPersomnCharacter|GetBP%20Third%20Person%20Character)) (+ (* (Math|Vector|Normalize (Math|Vector|GetForwardVector (Variables|/Game/ThirdPerson/Blueprints/BP_ThirdPersonCharacter.BP_ThirdPersonCharacter_C|GetFollowCamera (Variables|ThirdPersomnCharacter|GetBP%20Third%20Person%20Character)))) (Variables|GrappleForceImpulse|GetCamera%20force%20impulse)) (* (Math|Vector|Normalize (- (Variables|GrappleVariables|GetGrapple%20hit%20location) (Transformation|GetActorLocation (Variables|ThirdPersomnCharacter|GetBP%20Third%20Person%20Character)))) (Variables|GrappleForceImpulse|GetHook%20force%20impulse))) false))